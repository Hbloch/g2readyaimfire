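; BP_G2Pawn is a player pawn that lets the player equip, aim and fire a cannon through Enhanced Input.
; BeginPlay registers the input mapping with the local player subsystem.
; The equip action toggles between spawning a BP_CannonActor at the Hand transform, without attaching it, and destroying it.
; Aim input adds local pitch and yaw to the cannon after a validity check, while shoot calls its Shoot function unguarded.
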(event Input|EnhancedActionEvents|EnhancedInputActionInputAction_G2Player_EquipCannon
  (params (ActionValue :type Boolean) (ElapsedSeconds :type Float%20%28double-precision%29) (TriggeredSeconds :type Float%20%28double-precision%29) (InputAction :type Input%20Action%20Object%20Reference :default "/Game/Player/InputAction_G2Player_EquipCannon.InputAction_G2Player_EquipCannon"))
  ;[1 0.8102 0.4664] Get the cannon
  (bind _output_get (Variables|Default|SetisEquipped (not (Variables|Default|GetisEquipped))))
  (if _output_get
    (Development|PrintString "Hello")
    (bind _returnvalue (Game|SpawnActorfromClass "/Game/Cannon/BP_CannonActor.BP_CannonActor_C" (Transformation|GetWorldTransform (Variables|Default|GetHand)) "Undefined" "MultiplyWithRoot" 0 0))
    (Variables|Default|SetCannon _returnvalue)
    (else
      (Actor|DestroyActor (Variables|Default|GetCannon)))))

(event Input|EnhancedActionEvents|EnhancedInputActionInputAction_CannonAim
  (params (ActionValue :type Vector%202D%20Structure) (ElapsedSeconds :type Float%20%28double-precision%29) (TriggeredSeconds :type Float%20%28double-precision%29) (InputAction :type Input%20Action%20Object%20Reference :default "/Game/Cannon/InputAction_CannonAim.InputAction_CannonAim"))
  (bind _cannon (Variables|Default|GetCannon))
  ;[1 0.6892 0.9505] Use Mouse or Gamepad Left Thumbstick to Aim the cannon
  (Utilities|IsValid _cannon
    (:Is%20Valid
      (Transformation|AddActorLocalRotation _cannon (Math|Rotator|MakeRotator 0.0 (.x ActionValue) (.y ActionValue)) false false))
    (:Is%20Not%20Valid
      (Development|PrintString "Cannon not found"))))

(event Input|EnhancedActionEvents|EnhancedInputActionInputAction_CannonShoot
  (params (ActionValue :type Boolean) (ElapsedSeconds :type Float%20%28double-precision%29) (TriggeredSeconds :type Float%20%28double-precision%29) (InputAction :type Input%20Action%20Object%20Reference :default "/Game/Cannon/InputAction_CannonShoot.InputAction_CannonShoot"))
  ;[0.6214 1 0.9501] Use Left Mouse Button or Gamepad Special Right to Shoot the Bullet
  (Default|Shoot (Variables|Default|GetCannon))
  (Development|PrintString "Shoot"))

(event EventBeginPlay
  (bind _returnvalue (Game|GetPlayerController 0))
  (bind _returnvalue_2 (PlayerController|LocalPlayerSubsystems|GetEnhancedInputLocalPlayerSubsystem _returnvalue))
  ;[1 1 1] Get Mapping Context
  (Utilities|IsValid _returnvalue_2
    (:Is%20Valid
      (Input|AddMappingContext _returnvalue_2 0 0 "(bIgnoreAllPressedKeysUntilRelease=True,bForceImmediately=False,bNotifyUserSettings=False)"))
    (:Is%20Not%20Valid
      (Development|PrintString "No Player Controller found"))))

(fn ConstructionScript)